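; BP_Potion_Strength is a potion item, a child Blueprint that by its name grants a strength effect to the first-person player.
; Its DrinkPotion override prints a debug string, finds BP_FirstPersonCharacter with GetActorOfClass and sets that character's potion effect to a fixed enum entry.
; It then calls and returns the parent DrinkPotion, leaving the rest of the drinking behavior to the base class.
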(fn `DrinkPotion`
  (returns (Success :type Boolean))
  (`KismetSystemLibrary.PrintString` "Child")
  (bind _returnvalue (`GameplayStatics.GetActorOfClass` "/Game/FirstPerson/Blueprints/BP_FirstPersonCharacter.BP_FirstPersonCharacter_C"))
  (`/Game/FirstPerson/Blueprints/BP_FirstPersonCharacter.Set_Potion_Effect` _returnvalue "NewEnumerator0")
  (bind _success (`parent.DrinkPotion`))
  (return _success))

(fn `UserConstructionScript`
  (`parent.UserConstructionScript`))