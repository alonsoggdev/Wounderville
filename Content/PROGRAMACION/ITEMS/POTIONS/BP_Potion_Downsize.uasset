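; BP_Potion_Downsize is a potion item that shrinks a nearby object when used.
; UsePotion finds the first-person character and runs a small sphere overlap at its PotionChild location, filtered to BP_Object_Base actors.
; The first hit gets its Downsize function called, then the parent UsePotion runs, so the parent logic only executes when a valid target is found.
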(fn `UsePotion`
  (bind _returnvalue (`GameplayStatics.GetActorOfClass` "/Game/FirstPerson/Blueprints/BP_FirstPersonCharacter.BP_FirstPersonCharacter_C"))
  (bind (_outactors _returnvalue_2) (`KismetSystemLibrary.SphereOverlapActors` (`SceneComponent.K2_GetComponentLocation` (`/Game/FirstPerson/Blueprints/BP_FirstPersonCharacter.PotionChild` _returnvalue)) 20.0 (`|MakeArray` "ObjectTypeQuery1" "ObjectTypeQuery2" :!type "EObjectTypeQuery Enum") "/Game/PROGRAMACION/ITEMS/BP_Object_Base.BP_Object_Base_C"))
  (if _returnvalue_2
    (bind _asbp_object_base (cast `/Game/PROGRAMACION/ITEMS/BP_Object_Base` (`|GetArrayItem` _outactors)))
    (`/Game/PROGRAMACION/ITEMS/BP_Object_Base.Downsize` _asbp_object_base)
    (`parent.UsePotion`)))

(fn `UserConstructionScript`
  (`parent.UserConstructionScript`))