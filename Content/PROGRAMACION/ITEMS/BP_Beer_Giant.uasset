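; BP_Beer_Giant is a giant beer item variant that ends the demo after it is downsized.
; It overrides Downsize, runs the parent behavior, then starts a short timer that calls EndGame by function name.
; EndGame looks up BP_FirstPersonCharacter with GetActorOfClass and calls its EndDemo.
; The event graph and construction script add no logic of their own.
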(fn `Downsize`
  (`parent.Downsize`)
  (`KismetSystemLibrary.K2_SetTimer` null "EndGame" 4.0))

(fn `EndGame`
  (bind _returnvalue (`GameplayStatics.GetActorOfClass` "/Game/FirstPerson/Blueprints/BP_FirstPersonCharacter.BP_FirstPersonCharacter_C"))
  (`/Game/FirstPerson/Blueprints/BP_FirstPersonCharacter.EndDemo` _returnvalue))

(fn `UserConstructionScript`
  (`parent.UserConstructionScript`))