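; BP_MusicZone is a trigger zone that raises or lowers a music emotion as the first-person player enters and leaves.
; It finds BP_MusicManager in the level on BeginPlay.
; On entry, EmotionValue selects a soft boost for mid values or a full boost at 5, applied to the zone's Emotion.
; On exit, it soft-kills that Emotion regardless of value.
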(event `self.ReceiveBeginPlay`
  (bind _returnvalue (`GameplayStatics.GetActorOfClass` "/Game/PROGRAMACION/MUSIC/BP_MusicManager.BP_MusicManager_C"))
  (set `self.MusicManager` _returnvalue))

(event `self.TriggerArea.OnComponentBeginOverlap`
  (params (OverlappedComponent :type "PrimitiveComponent Object Reference") (OtherActor :type "Actor Object Reference") (OtherComp :type "PrimitiveComponent Object Reference") (OtherBodyIndex :type Integer) (bFromSweep :type Boolean) (SweepResult :type "HitResult Structure (by ref)"))
  (bind _musicmanager (`self.MusicManager`))
  (bind _emotion (`self.Emotion`))
  (cast `/Game/FirstPerson/Blueprints/BP_FirstPersonCharacter` OtherActor)
  (`/Engine/EditorBlueprintResources/StandardMacros.IsValid` _musicmanager
    (:`Is Valid`
      (switch `int` (`self.EmotionValue`)
        (:`3`
          (`/Game/PROGRAMACION/MUSIC/BP_MusicManager.SoftBoostEmotion` _musicmanager _emotion :!label _label))
        (:`4`
          (goto _label))
        (:`5`
          (`/Game/PROGRAMACION/MUSIC/BP_MusicManager.BoostEmotion` _musicmanager _emotion))))))

(event `self.TriggerArea.OnComponentEndOverlap`
  (params (OverlappedComponent :type "PrimitiveComponent Object Reference") (OtherActor :type "Actor Object Reference") (OtherComp :type "PrimitiveComponent Object Reference") (OtherBodyIndex :type Integer))
  (bind _musicmanager (`self.MusicManager`))
  (cast `/Game/FirstPerson/Blueprints/BP_FirstPersonCharacter` OtherActor)
  (`/Engine/EditorBlueprintResources/StandardMacros.IsValid` _musicmanager
    (:`Is Valid`
      (`/Game/PROGRAMACION/MUSIC/BP_MusicManager.SoftKillEmotion` _musicmanager (`self.Emotion`)))))

(fn `UserConstructionScript`)