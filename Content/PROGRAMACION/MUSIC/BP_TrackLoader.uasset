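; BP_TrackLoader is an actor that loads a list of music tracks and can play them by index.
; On BeginPlay, LoadTracks synchronously loads each AudioTracks path through a soft object path and writes the SoundWave back into its struct, keeping name, emotion and ambience data.
; A failed SoundWave cast has no fallback handling.
; PlayTrackInIndex plays the selected track's audio as a 2D sound.
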(event `self.ReceiveBeginPlay`
  (`self.LoadTracks`))

(fn `LoadTracks`
  (for (_array_element _array_index) (`self.AudioTracks`)
    (bind (_name _path _audio _emotions _ambience) (break `/Game/PROGRAMACION/DATA/STR_MusicTrack` _array_element))
    (bind _returnvalue (`KismetSystemLibrary.LoadAsset_Blocking` (`KismetSystemLibrary.Conv_SoftObjPathToSoftObjRef` (`KismetSystemLibrary.MakeSoftObjectPath` _path))))
    (bind _assound_wave (cast `SoundWave` _returnvalue))
    (`KismetArrayLibrary.Array_Set` (`self.AudioTracks`) _array_index (make `/Game/PROGRAMACION/DATA/STR_MusicTrack` _name _path _assound_wave _emotions _ambience))))

(fn `PlayTrackInIndex`
  (params (Index :type Integer))
  (`GameplayStatics.PlaySound2D` (`.Audio_14_CB75715E4C42D41DF5CF87B9CAB990AE` (break `/Game/PROGRAMACION/DATA/STR_MusicTrack` (`|GetArrayItem` (`self.AudioTracks`) Index))) 1.0 1.0 0.0 null null))

(fn `UserConstructionScript`)