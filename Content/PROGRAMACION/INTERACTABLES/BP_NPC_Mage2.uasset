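; BP_NPC_Mage2 is a child NPC Blueprint for the second mage, who provides the Bark of the Ancient Oak ingredient through dialogue.
; It overrides DialogueEndHandler: after the parent logic, ending dialogue index 2 spawns the ingredient and turns off its task mark.
; If Mage1's dialogue index is at least 2, it then changes Mage3's task mark sprite, finding both mages by class lookup.
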(fn `DialogueEndHandler`
  (params (`Dialogue Index` :type Integer))
  (`parent.DialogueEndHandler` `Dialogue Index`)
  (switch `int` `Dialogue Index`
    (:`2`
      (`self.SpawnIngredient` "/Game/PROGRAMACION/ITEMS/INGREDIENTS/BP_Ingredient_BarkOfTheAncientOak.BP_Ingredient_BarkOfTheAncientOak_C")
      (`self.SetTaskMarkActive` false)
      (bind _returnvalue (`GameplayStatics.GetActorOfClass` "/Game/PROGRAMACION/INTERACTABLES/BP_NPC_Mage1.BP_NPC_Mage1_C"))
      (if (>= (`/Game/PROGRAMACION/INTERACTABLES/BP_NPC.DialogueIndex` _returnvalue) 2)
        (bind _returnvalue_2 (`GameplayStatics.GetActorOfClass` "/Game/PROGRAMACION/INTERACTABLES/BP_NPC_Mage3.BP_NPC_Mage3_C"))
        (`self.SetTaskMarkSprite` _returnvalue_2 "NewEnumerator0")))))

(fn `UserConstructionScript`
  (`parent.UserConstructionScript`))