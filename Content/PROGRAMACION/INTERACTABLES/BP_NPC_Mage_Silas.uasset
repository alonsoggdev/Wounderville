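; Mage NPC Silas, who runs indexed dialogues and provides task helpers for a quest marker, ingredient spawning and player potion-inventory checks.
; EventDialogue steps through the current dialogue in the UI behind a resettable DoOnce, freezing player movement and camera until it finishes.
; Unless looping, completion calls DialogueEnd, whose handler only prints the index, then advances to the next dialogue.
; The task mark starts hidden and follows the player's yaw each tick.
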(event `self.ReceiveBeginPlay`
  (`self.SetTaskMarkActive` false))

(event `Dialogue End`
  (params (`Dialogue End` :type Integer))
  (`self.DialogueEndHandler` `Dialogue End`))

(event `self.ReceiveTick`
  (params (DeltaSeconds :type "Float (single-precision)"))
  (bind _taskmark (`self.TaskMark`))
  (bind (_returnvalue_roll _returnvalue_pitch) (`KismetMathLibrary.BreakRotator` (`SceneComponent.K2_GetComponentRotation` _taskmark)))
  (bind _returnvalue (`GameplayStatics.GetActorOfClass` "/Game/FirstPerson/Blueprints/BP_FirstPersonCharacter.BP_FirstPersonCharacter_C"))
  (bind (_returnvalue_roll_2 _returnvalue_pitch_2 _returnvalue_yaw) (`KismetMathLibrary.BreakRotator` (`self.K2_GetActorRotation` _returnvalue)))
  (`SceneComponent.K2_SetWorldRotation` _taskmark (`KismetMathLibrary.MakeRotator` _returnvalue_roll _returnvalue_pitch (+ _returnvalue_yaw 90.0)) false false))

(event `self.EventDialogue`
  (bind _dialogueui (`self.DialogueUI`))
  (bind _returnvalue (+ (`/Game/UI/UI_Dialogue.TextIndex` _dialogueui) 1))
  (`/Engine/EditorBlueprintResources/StandardMacros.DoOnce` false :!label _label
    (:`Completed`
      (bind _keys (`BlueprintMapLibrary.Map_Keys` (`self.Dialogues`)))
      (if (<= (`self.DialogueIndex`) (`KismetArrayLibrary.Array_Length` _keys))
        (`/Engine/EditorBlueprintResources/StandardMacros.IsValid` _dialogueui
          (:`Is Valid`
            (bind _output_get (set `self.CurrentDialogue` (`.Dialogue_3_339EC29543A6BB69A1C31CBB9C98A4BE` (break `/Game/PROGRAMACION/DATA/STR_Dialogue` (`BlueprintMapLibrary.Map_Find` (`self.Dialogues`) (`self.DialogueIndex`))))))
            (set `/Game/UI/UI_Dialogue.Text` _output_get _dialogueui)
            (`Widget.SetVisibility` (`/Game/UI/UI_Dialogue.TextDialogue` _dialogueui) "Visible")
            (`Widget.SetVisibility` (`/Game/UI/UI_Dialogue.DialogueBox` _dialogueui) "Visible")
            (`Widget.SetVisibility` (`/Game/UI/UI_Dialogue.CharacterImage` _dialogueui) "Visible")
            (`Image.SetBrushFromTexture` (`/Game/UI/UI_Dialogue.CharacterImage` _dialogueui) (`self.DialogueImage`) true)
            ; Termina el dialogo
            (if (> _returnvalue (- (`KismetArrayLibrary.Array_Length` (`self.CurrentDialogue`)) 1))
              (`Widget.RemoveFromParent` (`self.DialogueUI`))
              (`self.SetPlayerControls` true)
              (set `self.DialogueUI` null)
              (if (not (`self.LoopDialogue`))
                (`self.Dialogue End` (`self.DialogueIndex`))
                (`/Engine/EditorBlueprintResources/StandardMacros.IncrementInt` (`self.DialogueIndex`)
                  (:`  `
                    _)))
              (`self.ResetDoOnce`)
              (else
                (`self.SetPlayerControls` false)
                (set `/Game/UI/UI_Dialogue.TextIndex` _returnvalue (`self.DialogueUI`))
                (`self.ResetDoOnce`))))
          (:`Is Not Valid`
            (`KismetSystemLibrary.PrintString` "Dialogue UI invalid")))))))

(event `ResetDoOnce`
  (goto _label :!via `Reset`))

(fn `CheckPlayerHasPotions`
  (params (Potion :type "Array of /Game/PROGRAMACION/ITEMS/POTIONS/BP_Potion Class Reference"))
  (returns (Reuslt :type Boolean))
  (locals (Result :type Boolean))
  (bind _returnvalue (`GameplayStatics.GetActorOfClass` "/Game/FirstPerson/Blueprints/BP_FirstPersonCharacter.BP_FirstPersonCharacter_C"))
  (for _array_element Potion
    (bind _has_potion (`self.PlayerHasPotion` _array_element (`/Game/FirstPerson/Blueprints/BP_FirstPersonCharacter.PotionInventory` _returnvalue)))
    (if (not _has_potion)
      (return false)))
  (return true))

(fn `DialogueEndHandler`
  (params (`Dialogue Index` :type Integer))
  (`KismetSystemLibrary.PrintText` (`|FormatText` "Dialogue index: {0}" `Dialogue Index`)))

(fn `GoToDialogueIndex`
  (params (Index :type Integer))
  (bind _result (`/Engine/EditorBlueprintResources/StandardMacros.DecrementInt` Index)
    (:`  `
      (set `self.DialogueIndex` _result))))

(fn `GoToNextDialogue`
  (`/Engine/EditorBlueprintResources/StandardMacros.IncrementInt` (`self.DialogueIndex`)))

(fn `PlayerHasPotion`
  (params (InputPin :type "/Game/PROGRAMACION/ITEMS/POTIONS/BP_Potion Class Reference") (Array :type "Array of /Game/PROGRAMACION/ITEMS/POTIONS/BP_Potion Object Reference"))
  (returns (`Has Potion` :type Boolean))
  (for _array_element Array
    (if (`GameplayStatics.ObjectIsA` _array_element InputPin)
      (return true)))
  (return false))

(fn `SetLoopDialogue`
  (params (LoopDialogue :type Boolean))
  (set `self.LoopDialogue` LoopDialogue))

(fn `SetPlayerControls`
  (params (Active :type Boolean))
  (bind _returnvalue (`GameplayStatics.GetActorOfClass` "/Game/FirstPerson/Blueprints/BP_FirstPersonCharacter.BP_FirstPersonCharacter_C"))
  (if Active
    (set `/Game/FirstPerson/Blueprints/BP_FirstPersonCharacter.MovementSpeed` 1.0 _returnvalue)
    (set `/Game/FirstPerson/Blueprints/BP_FirstPersonCharacter.CameraSpeed` 1.0 _returnvalue)
    (else
      (set `/Game/FirstPerson/Blueprints/BP_FirstPersonCharacter.MovementSpeed` 0.0 _returnvalue)
      (set `/Game/FirstPerson/Blueprints/BP_FirstPersonCharacter.CameraSpeed` 0.0 _returnvalue))))

(fn `SetTaskMarkActive`
  (params (Active :type Boolean))
  (`SceneComponent.SetHiddenInGame` (`self.TaskMark`) (not Active) false))

(fn `SetTaskMarkSprite`
  (params (NewParam :type "/Game/PROGRAMACION/DATA/ENUM_NPC_TaskStatus Enum" :default "NewEnumerator0"))
  (bind _taskmark (`self.TaskMark`))
  (switch `/Game/PROGRAMACION/DATA/ENUM_NPC_TaskStatus` NewParam
    (:`NewEnumerator0`
      (`PaperSpriteComponent.SetSprite` _taskmark "/Game/ARTE/SPRITES/Sprites/HUD_Map_Task_Unactive_Sprite.HUD_Map_Task_Unactive_Sprite"))
    (:`NewEnumerator1`
      (`PaperSpriteComponent.SetSprite` _taskmark "/Game/ARTE/SPRITES/Sprites/HUD_Map_Task_Active_Sprite.HUD_Map_Task_Active_Sprite"))))

(fn `SpawnIngredient`
  (params (Ingredient :type "/Game/PROGRAMACION/ITEMS/INGREDIENTS/BP_Ingredient_Base Class Reference"))
  (`|SpawnActorFromClass` Ingredient (`SceneComponent.K2_GetComponentToWorld` (`self.ItemSpawnPoint`)) "Undefined" "MultiplyWithRoot" self null))

(fn `UserConstructionScript`)