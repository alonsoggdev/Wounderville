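; BP_Potion_Storage is an interactable that stores potions and spawns a copy of each one's class in the world.
; BeginPlay derives row and column capacity from the Cube's relative scale and spacing offsets.
; AddPotion records the potion, spawns at SpawnPoint, then steps it by both offsets, or resets X and advances the column at the row limit.
; CurrentRow never increments here, and Columns is never checked.
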(event `self.ReceiveBeginPlay`
  (set `self.Rows` (`KismetMathLibrary.FTrunc` (/ (.x (`SceneComponent.RelativeScale3D` (`self.Cube`))) (`self.OffsetX`))))
  (set `self.Columns` (`KismetMathLibrary.FTrunc` (/ (.y (`SceneComponent.RelativeScale3D` (`self.Cube`))) (`self.OffsetY`)))))

(event `Add Potion`
  (params (Potion :type "/Game/PROGRAMACION/ITEMS/POTIONS/BP_Potion Object Reference"))
  (`self.AddPotion` Potion))

(fn `AddPotion`
  (params (Potion :type "/Game/PROGRAMACION/ITEMS/POTIONS/BP_Potion Object Reference"))
  (`KismetArrayLibrary.Array_Add` (`self.PotionStorage`) Potion)
  (`|SpawnActorFromClass` (`GameplayStatics.GetObjectClass` Potion) (`KismetMathLibrary.Conv_VectorToTransform` (`self.SpawnPoint`)) "Undefined" "MultiplyWithRoot" null null)
  (if (>= (`self.CurrentRow`) (`self.Rows`))
    (set `self.SpawnPoint` (`KismetMathLibrary.MakeVector` 0.0 (+ (.y (`self.SpawnPoint`)) (`self.OffsetY`)) (.z (`self.SpawnPoint`))))
    (set `self.CurrentRow` 0)
    (bind _result (`/Engine/EditorBlueprintResources/StandardMacros.IncrementInt` (`self.CurrentColumn`))
      (:`  `
        (set `self.CurrentColumn` _result)))
    (else
      (set `self.SpawnPoint` (`KismetMathLibrary.MakeVector` (+ (.x (`self.SpawnPoint`)) (`self.OffsetX`)) (+ (.y (`self.SpawnPoint`)) (`self.OffsetY`)) (.z (`self.SpawnPoint`)))))))

(fn `UserConstructionScript`)