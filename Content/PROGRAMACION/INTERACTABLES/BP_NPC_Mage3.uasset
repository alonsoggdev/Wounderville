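; Third mage quest NPC whose dialogue tracks a strength potion task and a pumpkin task.
; A dialogue-end handler branches by index, checking the player's potions or whether the Pumpkin reference is still valid, then sets the next dialogue and task mark.
; Separately, the first time a heavy rock leaves BarrelTriggerOut, it moves BP_NPC_Mage4 to a hard-coded location.
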(event `self.ReceiveBeginPlay`
  (`parent.ReceiveBeginPlay`))

(event `self.BarrelTriggerOut.OnComponentEndOverlap`
  (params (OverlappedComponent :type "PrimitiveComponent Object Reference") (OtherActor :type "Actor Object Reference") (OtherComp :type "PrimitiveComponent Object Reference") (OtherBodyIndex :type Integer))
  (cast `/Game/PROGRAMACION/ITEMS/BP_Object_HeavyRock` OtherActor)
  (`/Engine/EditorBlueprintResources/StandardMacros.DoOnce` false
    (:`Completed`
      (bind _returnvalue (`GameplayStatics.GetActorOfClass` "/Game/PROGRAMACION/INTERACTABLES/BP_NPC_Mage4.BP_NPC_Mage4_C"))
      (`self.K2_SetActorLocation` _returnvalue (18042.788635 -5369.368776 876.481866) false false))))

(fn `DialogueEndHandler`
  (params (`Dialogue Index` :type Integer))
  (`parent.DialogueEndHandler` `Dialogue Index`)
  (switch `int` `Dialogue Index`
    (:`2`
      (bind _reuslt (`self.CheckPlayerHasPotions` (`|MakeArray` "/Game/PROGRAMACION/ITEMS/POTIONS/BP_Potion_Strength.BP_Potion_Strength_C" :!type "/Game/PROGRAMACION/ITEMS/POTIONS/BP_Potion Class Reference") :!label _label))
      (if _reuslt
        (`self.GoToDialogueIndex` 4)
        (else
          (`self.GoToDialogueIndex` 3)
          (`self.SetTaskMarkSprite` "NewEnumerator1"))))
    (:`3`
      (goto _label))
    (:`4`
      (`/Engine/EditorBlueprintResources/StandardMacros.IsValid` (`self.Pumpkin`)
        (:`Is Valid`
          (`self.GoToDialogueIndex` 4)
          (`self.SetTaskMarkSprite` "NewEnumerator1"))
        (:`Is Not Valid`
          (`self.GoToDialogueIndex` 5))))
    (:`5`
      (`self.SetTaskMarkActive` false))))

(fn `UserConstructionScript`
  (`parent.UserConstructionScript`))