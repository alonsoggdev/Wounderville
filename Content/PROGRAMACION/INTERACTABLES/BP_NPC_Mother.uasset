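; Mother NPC that starts the ingredient-collection tutorial through dialogue, built on a parent NPC class.
; It shows its task mark on BeginPlay, then reacts in DialogueEndHandler when a specific dialogue index ends.
; That step gives the first-person character two ingredient collection tasks, activates task marks on three Mage NPCs, pins their locations on the minimap and changes its own mark sprite.
; All targets are found with GetActorOfClass.
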(event `self.ReceiveBeginPlay`
  (`parent.ReceiveBeginPlay`)
  (`self.SetTaskMarkActive` true))

(fn `DialogueEndHandler`
  (params (`Dialogue Index` :type Integer))
  (`parent.DialogueEndHandler` `Dialogue Index`)
  (switch `int` `Dialogue Index`
    (:`5`
      (bind _returnvalue (`GameplayStatics.GetActorOfClass` "/Game/FirstPerson/Blueprints/BP_FirstPersonCharacter.BP_FirstPersonCharacter_C"))
      (`/Game/FirstPerson/Blueprints/BP_FirstPersonCharacter.AddTask` _returnvalue (make `/Game/PROGRAMACION/DATA/STR_TaskItem` false "/Game/PROGRAMACION/ITEMS/INGREDIENTS/BP_Ingredient_BarkOfTheAncientOak.BP_Ingredient_BarkOfTheAncientOak_C" "NewEnumerator1" 1 0 "Collect 1 Bark of the Ancient Oak" null))
      (`/Game/FirstPerson/Blueprints/BP_FirstPersonCharacter.AddTask` _returnvalue (make `/Game/PROGRAMACION/DATA/STR_TaskItem` false "/Game/PROGRAMACION/ITEMS/INGREDIENTS/BP_Ingredient_SummerbloomCarminOil.BP_Ingredient_SummerbloomCarminOil_C" "NewEnumerator1" 1 0 "Collect 1 Summerbloom Carmin Oil" null))
      (bind _returnvalue_2 (`GameplayStatics.GetActorOfClass` "/Game/PROGRAMACION/INTERACTABLES/BP_NPC_Mage1.BP_NPC_Mage1_C"))
      (`self.SetTaskMarkActive` _returnvalue_2 true)
      (bind _returnvalue_3 (`GameplayStatics.GetActorOfClass` "/Game/PROGRAMACION/INTERACTABLES/BP_NPC_Mage2.BP_NPC_Mage2_C"))
      (`self.SetTaskMarkActive` _returnvalue_3 true)
      (bind _returnvalue_4 (`GameplayStatics.GetActorOfClass` "/Game/PROGRAMACION/INTERACTABLES/BP_NPC_Mage3.BP_NPC_Mage3_C"))
      (`self.SetTaskMarkActive` _returnvalue_4 true)
      (bind _returnvalue_5 (`GameplayStatics.GetActorOfClass` "/Game/UI/MINIMAP/BP_Minimap.BP_Minimap_C"))
      (bind (_returnvalue_x _returnvalue_y) (`KismetMathLibrary.BreakVector` (`self.K2_GetActorLocation` _returnvalue_2)))
      (`/Game/UI/MINIMAP/BP_Minimap.AddPoint` _returnvalue_5 "NewEnumerator0" (`KismetMathLibrary.MakeVector2D` _returnvalue_x _returnvalue_y))
      (bind (_returnvalue_x_2 _returnvalue_y_2) (`KismetMathLibrary.BreakVector` (`self.K2_GetActorLocation` _returnvalue_3)))
      (`/Game/UI/MINIMAP/BP_Minimap.AddPoint` _returnvalue_5 "NewEnumerator0" (`KismetMathLibrary.MakeVector2D` _returnvalue_x_2 _returnvalue_y_2))
      (bind (_returnvalue_x_3 _returnvalue_y_3) (`KismetMathLibrary.BreakVector` (`self.K2_GetActorLocation` _returnvalue_4)))
      (`/Game/UI/MINIMAP/BP_Minimap.AddPoint` _returnvalue_5 "NewEnumerator0" (`KismetMathLibrary.MakeVector2D` _returnvalue_x_3 _returnvalue_y_3))
      (`self.SetTaskMarkSprite` "NewEnumerator1"))))

(fn `UserConstructionScript`
  (`parent.UserConstructionScript`))