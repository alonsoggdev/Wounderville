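; Task manager Blueprint that listens for item events to count down the item requirements of unlocked tasks.
; On BeginPlay it binds HandleTasks to the tasks event dispatcher, which passes the received item to HandleTaskEvents.
; That function loops over TasksArray, looks up the item in each unlocked task's Items map and decrements the found value.
; No explicit write-back to the map or completion check follows.
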(event `self.ReceiveBeginPlay`
  (add `self.Tasks_EventDispatcher` (delegate `Handle Tasks`)))

(event `Handle Tasks` :!signature `self.Tasks_EventDispatcher`
  (params (Item :type "/Game/PROGRAMACION/ITEMS/POTIONS/BP_Potion Object Reference"))
  (`self.HandleTaskEvents` Item))

(fn `HandleTaskEvents`
  (params (Item :type "/Game/PROGRAMACION/ITEMS/POTIONS/BP_Potion Object Reference"))
  (for _array_element (`self.Tasks_Array`)
    (bind (_items _day _unlocked) (break `/Game/PROGRAMACION/DATA/STR_Task` _array_element))
    (if _unlocked
      (bind (_value _returnvalue) (`BlueprintMapLibrary.Map_Find` _items Item))
      (if _returnvalue
        (`/Engine/EditorBlueprintResources/StandardMacros.DecrementInt` _value)))))

(fn `UserConstructionScript`)