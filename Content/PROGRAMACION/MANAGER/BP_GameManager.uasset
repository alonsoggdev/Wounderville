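; BP_GameManager builds a save object holding the current run's state.
; SaveGame creates a BP_SaveGame, finds the first-person character and maps each jar's first tag to its item count.
; It packs that map with current day, remaining day time, player position and inventory into RunSaveData.
; The function only fills the save buffer; it does not write to a slot.
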(fn `Save Game`
  (bind _playerreference (`self.PlayerReference`))
  (bind _returnvalue (`GameplayStatics.CreateSaveGameObject` "/Game/PROGRAMACION/MANAGER/BP_SaveGame.BP_SaveGame_C"))
  (set `self.SaveGameBuffer` _returnvalue)
  (bind _returnvalue_2 (`GameplayStatics.GetActorOfClass` "/Game/FirstPerson/Blueprints/BP_FirstPersonCharacter.BP_FirstPersonCharacter_C"))
  (set `self.PlayerReference` _returnvalue_2)
  (bind _outactors (`GameplayStatics.GetAllActorsOfClass` "/Game/PROGRAMACION/INTERACTABLES/BP_Item_Jar.BP_Item_Jar_C"))
  (for _array_element _outactors
    (`BlueprintMapLibrary.Map_Add` (`self.GM_ItemsInJars`) (`|GetArrayItem` (`Actor.Tags` _array_element)) (`KismetArrayLibrary.Array_Length` (`/Game/PROGRAMACION/INTERACTABLES/BP_Item_Jar.Items` _array_element))))
  (set `/Game/PROGRAMACION/MANAGER/BP_SaveGame.RunSaveData` (make `/Game/PROGRAMACION/DATA/STR_RunSaveData` (`self.GM_CurrentDay`) (`self.GM_DayTimeRemaining`) (`Actor.K2_GetActorLocation` _playerreference) (`/Game/FirstPerson/Blueprints/BP_FirstPersonCharacter.Inventory` _playerreference) (`self.GM_ItemsInJars`)) (`self.SaveGameBuffer`)))