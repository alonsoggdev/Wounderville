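; Actor component that lets the player focus and interact with BP_InteractionArea actors, either instantly or by holding input.
; Each tick it line-traces from the camera manager and toggles focus on the area hit, cancelling any interaction in progress when focus is lost.
; For timed areas, a looping timer fills the parent actor's round charge bar, with extra color and size effects for power charges.
; Completion sends an interface interact message to the area's parent actor.
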(event `self.ReceiveTick`
  (params (DeltaSeconds :type "Float (single-precision)"))
  (`self.Trace`))

(event `TryToInteract`
  (params (In :type Boolean))
  (if In
    (if (`self.IsTracingInterArea`)
      (bind _output_get (set `self.Interact Duration` (`/Game/ARTE/A_BLUEPRINTS/Interaction/InteractionArea/BP_InteractionArea.InteractDuration` (`self.FocusedInterArea`))))
      (if (> _output_get 0.0)
        (bind (_e_overlay _chargebar) (message `/Game/ARTE/A_BLUEPRINTS/Interaction/BI_Interaction.GetWidgetRef` (`Actor.GetParentActor` (`self.FocusedInterArea`))))
        (bind _aswbp_round_charge_bar (cast `/Game/UI/WBP_RoundChargeBar` (`WidgetComponent.GetWidget` _chargebar)))
        (set `self.CurrentInteractionWidgetGrafic` _aswbp_round_charge_bar)
        (bind _returnvalue (`KismetSystemLibrary.K2_SetTimerDelegate` (delegate `UpdateInteractionProgress`) (`self.UpdateFrameRate`) true))
        (set `self.InteractionTimer` _returnvalue)
        (else
          (`self.InteractOn` (`self.FocusedInterArea`)))))
    (else
      (`self.InteractionStop`))))

(event `UpdateInteractionProgress`
  (bind _interactionprogress (`self.InteractionProgress`))
  (bind _currentinteractionwidgetgrafic (`self.CurrentInteractionWidgetGrafic`))
  (bind _interact_duration (`self.Interact Duration`))
  (bind _output_get (set `self.InteractionProgress` (* (`self.Counter`) (* (/ 1.0 (`self.Interact Duration`)) (`self.UpdateFrameRate`)))))
  (`/Engine/EditorBlueprintResources/StandardMacros.IncrementFloat` (`self.Counter`)
    (:`  `
      (`/Game/UI/WBP_RoundChargeBar.SetPercent` (`self.CurrentInteractionWidgetGrafic`) _output_get)
      (if (`/Game/ARTE/A_BLUEPRINTS/Interaction/InteractionArea/BP_InteractionArea.PowerCharge` (`self.FocusedInterArea`))
        (`/Game/UI/WBP_RoundChargeBar.ChangeColor` _currentinteractionwidgetgrafic _interactionprogress _interact_duration)
        (`/Game/UI/WBP_RoundChargeBar.SetThickness` _currentinteractionwidgetgrafic _interactionprogress _interact_duration)
        (`/Game/UI/WBP_RoundChargeBar.SetSize` _currentinteractionwidgetgrafic _interactionprogress _interact_duration))
      (if (>= (`self.InteractionProgress`) 1.0)
        (`self.InteractionStop`)
        (`self.InteractOn` (`self.FocusedInterArea`))))))

(event `InteractOn`
  (params (InteractionArea :type "/Game/ARTE/A_BLUEPRINTS/Interaction/InteractionArea/BP_InteractionArea Object Reference"))
  (message `/Game/ARTE/A_BLUEPRINTS/Interaction/BI_Interaction.InterfaceInteract` (`Actor.GetParentActor` InteractionArea)))

(fn `InteractionStop`
  (bind _currentinteractionwidgetgrafic (`self.CurrentInteractionWidgetGrafic`))
  (if (> (`self.InteractionProgress`) 0.0)
    (`KismetSystemLibrary.K2_ClearAndInvalidateTimerHandle` (`self.InteractionTimer`))
    (`/Game/UI/WBP_RoundChargeBar.SetPercent` _currentinteractionwidgetgrafic 0.0)
    (`/Game/UI/WBP_RoundChargeBar.ResetColor` _currentinteractionwidgetgrafic)
    (`/Game/UI/WBP_RoundChargeBar.SetThickness` _currentinteractionwidgetgrafic 0.0 0.0)
    (set `self.InteractionProgress` 0.0)
    (set `self.CurrentInteractionWidgetGrafic` null)
    (set `self.Counter` 0.0)))

(fn `Trace`
  (bind _returnvalue (`GameplayStatics.GetPlayerCameraManager` 0))
  (bind _returnvalue_2 (`Actor.K2_GetActorLocation` _returnvalue))
  (bind (_outhit _returnvalue_3) (`KismetSystemLibrary.LineTraceSingle` :`Start` _returnvalue_2 :`End` (+ _returnvalue_2 (* (`KismetMathLibrary.GetForwardVector` (`Actor.K2_GetActorRotation` _returnvalue)) (`self.Length`))) :`TraceChannel` "TraceTypeQuery1" :`TraceColor` (struct :`G` 1.0 :`B` 0.623003 :`A` 1.0) :`TraceHitColor` (struct :`R` 1.0 :`G` 0.178356 :`A` 1.0)))
  (if _returnvalue_3
    (bind (_bblockinghit _binitialoverlap _time _distance _location _impactpoint _normal _impactnormal _physmat _hitactor) (`GameplayStatics.BreakHitResult` _outhit))
    (if (!= (`self.FocusedActor`) _hitactor)
      (set `self.FocusedActor` _hitactor)
      (`self.TraceInteractionArea` (== (`GameplayStatics.GetObjectClass` _hitactor) "/Game/ARTE/A_BLUEPRINTS/Interaction/InteractionArea/BP_InteractionArea.BP_InteractionArea_C")))
    (else
      (`self.TraceInteractionArea` false))))

(fn `TraceInteractionArea`
  (params (Trace :type Boolean))
  (if Trace
    (if (`self.IsTracingInterArea`)
      (`/Game/ARTE/A_BLUEPRINTS/Interaction/InteractionArea/BP_InteractionArea.ToggleFocus` (`self.FocusedInterArea`) false))
    (bind _asbp_interaction_area (cast `/Game/ARTE/A_BLUEPRINTS/Interaction/InteractionArea/BP_InteractionArea` (`self.FocusedActor`)))
    (bind _output_get (set `self.FocusedInterArea` _asbp_interaction_area))
    (`/Game/ARTE/A_BLUEPRINTS/Interaction/InteractionArea/BP_InteractionArea.ToggleFocus` _output_get true)
    (set `self.IsTracingInterArea` true)
    (elif (`self.IsTracingInterArea`)
      (`/Engine/EditorBlueprintResources/StandardMacros.IsValid` (`self.FocusedInterArea`)
        (:`Is Valid`
          (`/Game/ARTE/A_BLUEPRINTS/Interaction/InteractionArea/BP_InteractionArea.ToggleFocus` (`self.FocusedInterArea`) false))
        (:`Is Not Valid`
          _))
      (set `self.IsTracingInterArea` false)
      (set `self.FocusedActor` null)
      (set `self.FocusedInterArea` null)
      (`self.InteractionStop`))))