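; Base interactable actor for pickups, with a press-E overlay widget and a carrot pickup popup, both starting hidden.
; Interface calls toggle custom depth on focus and trigger interaction, which flips a RepNotify toggle, then destroys the actor after a delay.
; The RepNotify plays the popup fade and pop sound and hides the mesh, prompt and child actor.
; GetWidgetRef exposes the prompt and charge bar.
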(event `self.ReceiveBeginPlay`
  (`|ExecutionSequence`
    (:`then_0`
      (bind _returnvalue (`|CreateWidget` "/Game/UI/WBP_InteractionOverlay.WBP_InteractionOverlay_C"))
      (bind _output_get (set `self.PressEWidget` _returnvalue))
      (`WidgetComponent.SetWidget` (`self.PressE`) _output_get)
      (bind _pressewidget (`self.PressEWidget`)
        (:`then`
          (`UserWidget.PlayAnimation` _pressewidget (`/Game/UI/WBP_InteractionOverlay.Hidden` _pressewidget) 0.0 1 "Forward" 1.0 false))
        (:`else`)))
    (:`then_1`
      (bind _returnvalue_2 (`|CreateWidget` "/Game/UI/WBP_PickUpCarrot.WBP_PickUpCarrot_C"))
      (bind _output_get_2 (set `self.OneUp` _returnvalue_2))
      (`WidgetComponent.SetWidget` (`self.+Carrot`) _output_get_2)
      (bind _oneup (`self.OneUp`)
        (:`then`
          (`UserWidget.PlayAnimation` _oneup (`/Game/UI/WBP_PickUpCarrot.Hidden` _oneup) 0.0 1 "Forward" 1.0 false))
        (:`else`)))))

(event `/Game/ARTE/A_BLUEPRINTS/Interaction/BI_Interaction.Interface_ToggleFocus`
  (params (Focus :type Boolean))
  (`PrimitiveComponent.SetRenderCustomDepth` (`self.StaticMesh`) Focus))

(event `/Game/ARTE/A_BLUEPRINTS/Interaction/BI_Interaction.InterfaceInteract`
  (`self.InteractOn`))

(event `InteractOn`
  (set `self.InteractionToggle` (not (`self.InteractionToggle`)))
  (`KismetSystemLibrary.Delay` (`self.InteractionLength`))
  (`self.K2_DestroyActor`))

(fn `GetWidgetRef`
  (returns (`E Overlay` :type "WidgetComponent Object Reference") (ChargeBar :type "WidgetComponent Object Reference"))
  (locals (NewLocalVar :type "WidgetComponent Object Reference"))
  (return (`self.PressE`) (`self.ChargeBar`)))

(fn `OnRep_InteractionOn`)

(fn `OnRep_InteractionToggle`
  (bind _returnvalue (`|CreateWidget` "/Game/UI/WBP_PickUpCarrot.WBP_PickUpCarrot_C"))
  (bind _output_get (set `self.OneUp` _returnvalue))
  (`WidgetComponent.SetWidget` (`self.+Carrot`) _output_get)
  (bind _oneup (`self.OneUp`)
    (:`then`
      (`UserWidget.PlayAnimation` _oneup (`/Game/UI/WBP_PickUpCarrot.Fade` _oneup) 0.0 1 "Forward" 1.5 false)
      (`GameplayStatics.PlaySoundAtLocation` "/Game/MUSIC/pop-268648.pop-268648" (`SceneComponent.GetSocketLocation` (`self.StaticMesh`) "None") (struct) 1.0 1.0 0.0 null null null null)
      (`SceneComponent.SetHiddenInGame` (`self.StaticMesh`) true false)
      (`SceneComponent.SetHiddenInGame` (`self.PressE`) true false)
      (`SceneComponent.SetHiddenInGame` (`self.ChildActor`) true false))
    (:`else`)))

(fn `UserConstructionScript`)