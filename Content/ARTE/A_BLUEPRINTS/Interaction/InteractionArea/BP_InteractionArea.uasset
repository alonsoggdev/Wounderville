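; BP_InteractionArea is an interaction-area Blueprint that relays focus changes to its parent actor and shows overlay feedback.
; ToggleFocus stores the state, forwards it through an interface message, and gets the parent's widget reference the same way.
; It creates a new WBP_InteractionOverlay on every toggle, sets it on the EOverlay returned by the parent, then plays Pop on focus or Fade otherwise.
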(event `ToggleFocus`
  (params (Focused :type Boolean))
  (set `self.Focused` Focused)
  (message `/Game/ARTE/A_BLUEPRINTS/Interaction/BI_Interaction.Interface_ToggleFocus` (`self.GetParentActor`) (`self.Focused`))
  (bind _e_overlay (message `/Game/ARTE/A_BLUEPRINTS/Interaction/BI_Interaction.GetWidgetRef` (`self.GetParentActor`)))
  (bind _returnvalue (`|CreateWidget` "/Game/UI/WBP_InteractionOverlay.WBP_InteractionOverlay_C"))
  (bind _output_get (set `self.OverlayWidget` _returnvalue))
  (`WidgetComponent.SetWidget` _e_overlay _output_get)
  (if (`self.Focused`)
    (bind _overlaywidget (`self.OverlayWidget`)
      (:`then`
        (`UserWidget.PlayAnimation` _overlaywidget (`/Game/UI/WBP_InteractionOverlay.Pop` _overlaywidget) 0.0 1 "Forward" 1.0 false))
      (:`else`))
    (else
      (bind _overlaywidget_2 (`self.OverlayWidget`)
        (:`then`
          (`UserWidget.PlayAnimation` _overlaywidget_2 (`/Game/UI/WBP_InteractionOverlay.Fade` _overlaywidget_2) 0.0 1 "Forward" 1.0 false))
        (:`else`)))))

(fn `UserConstructionScript`)